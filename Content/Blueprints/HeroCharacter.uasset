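; Player hero character with axis-driven world-space movement, look-to-fire shooting, health and item use.
; On BeginPlay it spawns a weapon attached at TempWeaponLocation, and destroys it along with the character.
; Both look axes share one branch that sets control rotation and pulls the trigger past a deadzone, otherwise releasing it.
; AffectHealth recalculates and prints health, while overlapping actors implementing the Usable interface are used by the hero.
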(event `self.ReceiveBeginPlay`
  (bind _temp_weaponlocation (`self.Temp_WeaponLocation`))
  (`|ExecutionSequence`
    (:`then_0`
      ;[1 1 1] Weapon Spawning
      (bind _returnvalue (`|SpawnActorFromClass` "/Game/Blueprints/Weapon.Weapon_C" (`SceneComponent.K2_GetComponentToWorld` _temp_weaponlocation) "Undefined" "OverrideRootScale" null null))
      (bind _output_get (set `self.Weapon` _returnvalue))
      (`self.K2_AttachToComponent` _output_get _temp_weaponlocation "None" "KeepWorld" "KeepWorld" "KeepWorld" true))))

(event `self.ReceiveDestroyed`
  (`self.K2_DestroyActor` (`self.Weapon`)))

(event `InputAxis|Vertical`
  (params (AxisValue :type "Float (single-precision)"))
  ;[1 1 1] Movement
  (`self.AddMovementInput` (1.0 0.0 0.0) AxisValue))

(event `InputAxis|Horizontal`
  (params (AxisValue :type "Float (single-precision)"))
  ;[1 1 1] Movement
  (`self.AddMovementInput` (0.0 1.0 0.0) AxisValue))

(event `InputAxis|LookVertical`
  (params (AxisValue :type "Float (single-precision)"))
  (bind _weapon (`self.Weapon`))
  ;[1 1 1] Rotation
  (bind _returnvalue (`KismetMathLibrary.MakeVector` AxisValue (stale `InputAxis|LookHorizontal` AxisValue)))
  (if (> (`KismetMathLibrary.VSize` _returnvalue) 0.25) :!label _label
    (`Controller.SetControlRotation` (`self.GetController`) (`KismetMathLibrary.Conv_VectorToRotator` _returnvalue))
    (`/Game/Blueprints/Weapon.PullTrigger` _weapon)
    (else
      (`/Game/Blueprints/Weapon.ReleaseTrigger` _weapon))))

(event `InputAxis|LookHorizontal`
  (params (AxisValue :type "Float (single-precision)"))
  ;[1 1 1] Rotation
  (goto _label))

(event `self.AffectHealth`
  (params (delta :type "Float (single-precision)"))
  ;[1 1 1] Damage
  (`self.CalculateHealth` delta)
  (`KismetSystemLibrary.PrintString` (`KismetStringLibrary.Conv_DoubleToString` (`self.Health`)) true true (struct :`G` 0.66 :`B` 1.0 :`A` 1.0) 1.0))

(event `self.ReceiveActorBeginOverlap`
  (params (OtherActor :type "Actor Object Reference"))
  (if (`KismetSystemLibrary.DoesImplementInterface` OtherActor "/Script/TwinStickShooter.Usable")
    (message `Usable.UseBy` OtherActor self)))

(fn `UserConstructionScript`)