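; Enemy character Blueprint that takes health changes and has a chance to spawn a configurable actor when it dies.
; AffectHealth recalculates and prints health, destroying the actor when dead; the bound death handler rolls against SpawnOnDiedPercentage to spawn at its transform.
; The construction script passes DamageVolume to the DamageOnCollisionOverlap component and tints the mesh through a dynamic material's BodyColor parameter.
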(event `self.ReceiveBeginPlay`
  (add `self.OnCharacterDied` (delegate `HandleOnDied`)))

(event `HandleOnDied`
  ;[1 1 1] Spawn Actor On Died
  (`/Engine/EditorBlueprintResources/StandardMacros.CompareFloat` (`self.SpawnOnDiedPercentage`) (`KismetMathLibrary.RandomFloatInRange` 0.0 1.0)
    (:`>`
      _)
    (:`==`
      _))
  (`|SpawnActorFromClass` (`self.ClassTypeToSpawnOnDied`) (`self.GetTransform`) "AlwaysSpawn" "OverrideRootScale" null null))

(event `self.AffectHealth`
  (params (delta :type "Float (single-precision)"))
  (`self.CalculateHealth` delta)
  (`KismetSystemLibrary.PrintString` (`KismetStringLibrary.Conv_DoubleToString` (`self.Health`)))
  (if (`self.IsDead`)
    (`self.K2_DestroyActor`)))

(fn `UserConstructionScript`
  (`|ExecutionSequence`
    (:`then_0`
      (set `DamageOnCollisionOverlap.CollisionComponent` (`self.DamageVolume`) (`self.DamageOnCollisionOverlap`)))
    (:`then_1`
      (bind _returnvalue (`PrimitiveComponent.CreateDynamicMaterialInstance` (`self.Mesh`) 0 null "None"))
      (bind _output_get (set `self.DynamicMaterial` _returnvalue))
      (`MaterialInstanceDynamic.SetVectorParameterValue` _output_get "BodyColor" (`self.BodyColor`)))))