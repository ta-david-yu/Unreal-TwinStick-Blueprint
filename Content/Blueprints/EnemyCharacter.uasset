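; Enemy character that takes damage, is destroyed when dead, and repeatedly damages overlapping IDamageable actors carrying DamageTag.
; AffectHealth updates and prints health, then destroys the actor if dead.
; Overlap starts a looping HitTarget timer paced by AttacksPerSecond; any overlap end clears it, as the target comparison is unwired.
; The construction script applies BodyColor through a dynamic material instance.
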(event `self.AffectHealth`
  (params (delta :type "Float (single-precision)"))
  (`self.CalculateHealth` delta)
  (`KismetSystemLibrary.PrintString` (`KismetStringLibrary.Conv_DoubleToString` (`self.Health`)))
  (if (`self.IsDead`)
    (`self.K2_DestroyActor`)))

(event `self.ReceiveActorBeginOverlap`
  (params (OtherActor :type "Actor Object Reference"))
  (if (`KismetSystemLibrary.DoesImplementInterface` OtherActor "/Script/TwinStickShooter.IDamageable")
    (if (`self.ActorHasTag` OtherActor (`self.DamageTag`))
      (bind _asidamageable (cast `IDamageable` OtherActor))
      (set `self.DamageTarget` _asidamageable)
      (`KismetSystemLibrary.K2_SetTimerDelegate` (delegate `HitTarget`) (/ 1.0 (`self.AttacksPerSecond`)) true))))

(event `HitTarget`
  ;[1 1 1] Hit Target (Damaging)
  (`IDamageable.AffectHealth` (`self.DamageTarget`) (`self.DamageHealthDelta`)))

(event `self.ReceiveActorEndOverlap`
  (params (OtherActor :type "Actor Object Reference"))
  ;[1 1 1] Clear HitTarget Timer
  (if true
    (`KismetSystemLibrary.K2_ClearTimer` null "HitTarget")))

(fn `UserConstructionScript`
  (bind _returnvalue (`PrimitiveComponent.CreateDynamicMaterialInstance` (`self.Mesh`) 0 null "None"))
  (bind _output_get (set `self.DynamicMaterial` _returnvalue))
  (`MaterialInstanceDynamic.SetVectorParameterValue` _output_get "BodyColor" (`self.BodyColor`)))